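; BP_Button is a pressable button that the player character can interact with while standing in its trigger box.
; Box overlap sets or clears itself as BP_PRSCharacter's InteractableActor and toggles interaction.
; On the bound press event, a timeline animates the inner cube's X scale to show it being pushed.
; If RePressable, the timeline reverses when finished, then calls ResetButton once back at the start.
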(event OnComponentBeginOverlap(Box)
  (params (OverlappedComponent :type Primitive%20Component%20Object%20Reference) (OtherActor :type Actor%20Object%20Reference) (OtherComp :type Primitive%20Component%20Object%20Reference) (OtherBodyIndex :type Integer) (bFromSweep :type Boolean) (SweepResult :type Hit%20Result%20Structure%20%28by%20ref%29))
  (bind _asbp_prscharacter (Utilities|Casting|CastToBP_PRSCharacter OtherActor))
  (Variables|/Script/Perspective.PRSCharacter|SetInteractableActor _asbp_prscharacter self)
  (Class|PRSInteractableActor|EnableInteraction))

(event OnComponentEndOverlap(Box)
  (params (OverlappedComponent :type Primitive%20Component%20Object%20Reference) (OtherActor :type Actor%20Object%20Reference) (OtherComp :type Primitive%20Component%20Object%20Reference) (OtherBodyIndex :type Integer))
  (bind _asbp_prscharacter (Utilities|Casting|CastToBP_PRSCharacter OtherActor))
  (Class|PRSInteractableActor|DisableInteraction)
  (Variables|/Script/Perspective.PRSCharacter|SetInteractableActor _asbp_prscharacter 0))

(event Custom|ButtonPressed
  (Development|PrintString "Pressed")
  (bind (_direction _scale3d_x_value) (Timeline|InnerCubePushedTimeline Play)
    (:Update
      (Transformation|SetRelativeScale3D (Variables|Default|GetInnerCubeScene) (Math|Vector|MakeVector _scale3d_x_value 1.0 1.0)))
    (:Finished
      (if (and (Utilities|Enum|Equal(Enum) _direction "Forward") (Variables|Default|GetbRePressable))
        (Timeline|InnerCubePushedTimeline Reverse)
        (elif (and (Utilities|Enum|Equal(Enum) _direction "Backward") (Variables|Default|GetbRePressable))
          (Class|PRSInteractableButton|ResetButton))))))

(event EventBeginPlay
  (EventDispatchers|BindEventtoOnButtonPressed (delegate Custom|ButtonPressed)))

(fn ConstructionScript)