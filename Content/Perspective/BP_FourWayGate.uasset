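; BP_FourWayGate is a four-sided gate that switches perspective mode when the perspective character passes through it.
; End-overlaps on the four side boxes, combined with the center box's touch state, determine entry or exit and record its side.
; Exiting by a different side than entered overrides the character's forward vector with that side box's, calls Switch on PerspectiveModeWorldSubsystem and plays a sound.
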(event OnComponentEndOverlap(BoxFront)
  (params (OverlappedComponent :type Primitive%20Component%20Object%20Reference) (OtherActor :type Actor%20Object%20Reference) (OtherComp :type Primitive%20Component%20Object%20Reference) (OtherBodyIndex :type Integer))
  (bind _asbp_perspective_character (Utilities|Casting|CastToBP_PerspectiveCharacter OtherActor))
  (if (CallFunction|Entered)
    (Variables|Default|SetIsInside true)
    (Variables|Default|SetEnterDirection 0)
    (elif (CallFunction|Exited)
      (Variables|Default|SetIsInside false)
      (Variables|Default|SetExitDirection 0)
      (CallFunction|Exit _asbp_perspective_character))))

(event OnComponentEndOverlap(BoxBack)
  (params (OverlappedComponent :type Primitive%20Component%20Object%20Reference) (OtherActor :type Actor%20Object%20Reference) (OtherComp :type Primitive%20Component%20Object%20Reference) (OtherBodyIndex :type Integer))
  (bind _asbp_perspective_character (Utilities|Casting|CastToBP_PerspectiveCharacter OtherActor))
  (if (CallFunction|Entered)
    (Variables|Default|SetIsInside true)
    (Variables|Default|SetEnterDirection 1)
    (elif (CallFunction|Exited)
      (Variables|Default|SetIsInside false)
      (Variables|Default|SetExitDirection 1)
      (CallFunction|Exit _asbp_perspective_character))))

(event OnComponentEndOverlap(BoxRight)
  (params (OverlappedComponent :type Primitive%20Component%20Object%20Reference) (OtherActor :type Actor%20Object%20Reference) (OtherComp :type Primitive%20Component%20Object%20Reference) (OtherBodyIndex :type Integer))
  (bind _asbp_perspective_character (Utilities|Casting|CastToBP_PerspectiveCharacter OtherActor))
  (if (CallFunction|Entered)
    (Variables|Default|SetIsInside true)
    (Variables|Default|SetEnterDirection 2)
    (elif (CallFunction|Exited)
      (Variables|Default|SetIsInside false)
      (Variables|Default|SetExitDirection 2)
      (CallFunction|Exit _asbp_perspective_character))))

(event OnComponentEndOverlap(BoxLeft)
  (params (OverlappedComponent :type Primitive%20Component%20Object%20Reference) (OtherActor :type Actor%20Object%20Reference) (OtherComp :type Primitive%20Component%20Object%20Reference) (OtherBodyIndex :type Integer))
  (bind _asbp_perspective_character (Utilities|Casting|CastToBP_PerspectiveCharacter OtherActor))
  (if (CallFunction|Entered)
    (Variables|Default|SetIsInside true)
    (Variables|Default|SetEnterDirection 3)
    (elif (CallFunction|Exited)
      (Variables|Default|SetIsInside false)
      (Variables|Default|SetExitDirection 3)
      (CallFunction|Exit _asbp_perspective_character))))

(event OnComponentBeginOverlap(BoxCenter)
  (params (OverlappedComponent :type Primitive%20Component%20Object%20Reference) (OtherActor :type Actor%20Object%20Reference) (OtherComp :type Primitive%20Component%20Object%20Reference) (OtherBodyIndex :type Integer) (bFromSweep :type Boolean) (SweepResult :type Hit%20Result%20Structure%20%28by%20ref%29))
  (Utilities|Casting|CastToBP_PerspectiveCharacter OtherActor)
  (Variables|Default|SetIsTouchingInside true))

(event OnComponentEndOverlap(BoxCenter)
  (params (OverlappedComponent :type Primitive%20Component%20Object%20Reference) (OtherActor :type Actor%20Object%20Reference) (OtherComp :type Primitive%20Component%20Object%20Reference) (OtherBodyIndex :type Integer))
  (Utilities|Casting|CastToBP_PerspectiveCharacter OtherActor)
  (Variables|Default|SetIsTouchingInside false))

(fn ConstructionScript)

(fn Exit
  (params (Character :type BP%20Perspective%20Character%20Object%20Reference))
  (if (!= (Variables|Default|GetEnterDirection) (Variables|Default|GetExitDirection))
    (Variables|/Script/Perspective.PerspectiveCharacter|SetForwardVectorOverride Character (CallFunction|DecideForwardVector))
    (Class|PerspectiveModeWorldSubsystem|Switch (Subsystems|GetPerspectiveModeWorldSubsystem))
    (Audio|PlaySound2D "/Game/Perspective/Assets/Sounds/A_PerspectiveModeChanged.A_PerspectiveModeChanged" 1.0 1.0 0.25 0 0)))

(fn DecideForwardVector
  (switch int (Variables|Default|GetExitDirection)
    (:0
      (return (Math|Vector|GetForwardVector (Variables|Default|GetBoxFront))))
    (:1
      (return (Math|Vector|GetForwardVector (Variables|Default|GetBoxBack))))
    (:2
      (return (Math|Vector|GetForwardVector (Variables|Default|GetBoxRight))))
    (:3
      (return (Math|Vector|GetForwardVector (Variables|Default|GetBoxLeft))))))

(fn Entered
  (return (and (not (Variables|Default|GetIsInside)) (Variables|Default|GetIsTouchingInside))))

(fn Exited
  (return (and (Variables|Default|GetIsInside) (not (Variables|Default|GetIsTouchingInside)))))