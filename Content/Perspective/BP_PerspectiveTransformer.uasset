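; BP_PerspectiveTransformer is a trigger volume that switches the world between 2D and 3D perspective when a PerspectiveCharacter passes through it.
; On overlap begin and end, it rounds the normalized offset from its center to the character into a flat X/Y direction.
; If exit and entry directions differ, it calls Switch on PerspectiveModeWorldSubsystem.
; When leaving 3D mode, it first sets the character's ForwardVectorOverride to the exit direction.
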(event OnComponentEndOverlap(Box)
  (params (OverlappedComponent :type Primitive%20Component%20Object%20Reference) (OtherActor :type Actor%20Object%20Reference) (OtherComp :type Primitive%20Component%20Object%20Reference) (OtherBodyIndex :type Integer))
  (bind _asperspective_character (Utilities|Casting|CastToPerspectiveCharacter OtherActor))
  (Variables|Default|SetExitDirection (CallFunction|DetermineOverlappingDirection (Transformation|GetActorLocation _asperspective_character)))
  (if (Utilities|Operators|NotEqual(!=) (Variables|Default|GetEnterDirection) (Variables|Default|GetExitDirection) 0.0)
    (switch Utilities|FlowControl|Switch|SwitchonEPerspectiveMode (Class|PerspectiveModeWorldSubsystem|GetMode (Subsystems|GetPerspectiveModeWorldSubsystem))
      (:TwoDimensional
        _)
      (:ThreeDimensional
        (Variables|/Script/Perspective.PerspectiveCharacter|SetForwardVectorOverride _asperspective_character (Variables|Default|GetExitDirection))))
    (Class|PerspectiveModeWorldSubsystem|Switch (Subsystems|GetPerspectiveModeWorldSubsystem))))

(event OnComponentBeginOverlap(Box)
  (params (OverlappedComponent :type Primitive%20Component%20Object%20Reference) (OtherActor :type Actor%20Object%20Reference) (OtherComp :type Primitive%20Component%20Object%20Reference) (OtherBodyIndex :type Integer) (bFromSweep :type Boolean) (SweepResult :type Hit%20Result%20Structure%20%28by%20ref%29))
  (bind _asperspective_character (Utilities|Casting|CastToPerspectiveCharacter OtherActor))
  (Variables|Default|SetEnterDirection (CallFunction|DetermineOverlappingDirection (Transformation|GetActorLocation _asperspective_character))))

(fn ConstructionScript)

(fn DetermineOverlappingDirection
  (params (OverlappingActorLocation :type Vector))
  (bind _returnvalue (Transformation|GetActorLocation))
  (bind _returnvalue_2 (- OverlappingActorLocation _returnvalue))
  (bind _returnvalue_3 (Math|Vector|Normalize _returnvalue_2))
  (return (Math|Vector|MakeVector (Math|Conversions|ToFloat(Integer) (Math|Float|Round (.x _returnvalue_3))) (Math|Conversions|ToFloat(Integer) (Math|Float|Round (.y _returnvalue_3))) 0.0)))