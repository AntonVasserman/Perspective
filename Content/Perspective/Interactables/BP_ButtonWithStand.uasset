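; Interactable push button on a stand that animates when pressed and can optionally be pressed again.
; A successful interaction plays a timeline that scales the Push component on Z, and a reset request reverses it.
; When RePressable, the button calls for a reset after the forward animation and tries to re-enable interaction after the reverse.
; Highlighting toggles custom depth on the Ring, using a stencil value set at BeginPlay, only while interactable.
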(event Custom|InteractionSucceeded
  (bind (_direction _scale3d_value) (Timeline|InnerCubePushedTimeline Play)
    (:Update
      (Transformation|SetRelativeScale3D (Variables|Default|GetPush) (Math|Vector|MakeVector 1.0 1.0 _scale3d_value)))
    (:Finished
      (switch Utilities|FlowControl|Switch|SwitchonETimelineDirection _direction
        (:Forward
          (if (Variables|Default|GetbRePressable)
            (Class|PRSInteractableButton|ResetButton)))
        (:Backward
          (if (Variables|Default|GetbRePressable)
            (Class|PRSInteractableButton|TryEnableInteraction)))))))

(event Custom|ResetButtonRequested
  (bind (_direction _scale3d_value) (Timeline|InnerCubePushedTimeline Reverse)
    (:Update
      (Transformation|SetRelativeScale3D (Variables|Default|GetPush) (Math|Vector|MakeVector 1.0 1.0 _scale3d_value)))
    (:Finished
      (switch Utilities|FlowControl|Switch|SwitchonETimelineDirection _direction
        (:Forward
          (if (Variables|Default|GetbRePressable)
            (Class|PRSInteractableButton|ResetButton)))
        (:Backward
          (if (Variables|Default|GetbRePressable)
            (Class|PRSInteractableButton|TryEnableInteraction)))))))

(event EventBeginPlay
  (EventDispatchers|BindEventtoOnInteractionSucceeded (EventDispatchers|CreateEvent :!event Custom|InteractionSucceeded))
  (EventDispatchers|BindEventtoOnResetButtonRequested (EventDispatchers|CreateEvent :!event Custom|ResetButtonRequested))
  (Rendering|SetCustomDepthStencilValue (Variables|Default|GetRing) 250))

(event EventHighlightImplementation
  (Rendering|SetRenderCustomDepth (Variables|Default|GetRing) (Class|PRSInteractableActor|IsInteractable)))

(event EventUnHighlightImplementation
  (Rendering|SetRenderCustomDepth (Variables|Default|GetRing) false))

(fn ConstructionScript)