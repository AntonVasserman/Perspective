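; Colored key pickup that the player collects, registering its color with the colored door world subsystem.
; When a PRSCharacter overlaps its sphere and a color is set, it adds the key, plays a pickup sound and destroys itself.
; The construction script picks the mesh material from the Color variable.
; Tick bobs the key vertically around its spawn location with a cosine of game time.
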(event OnComponentBeginOverlap(Sphere)
  (params (OverlappedComponent :type Primitive%20Component%20Object%20Reference) (OtherActor :type Actor%20Object%20Reference) (OtherComp :type Primitive%20Component%20Object%20Reference) (OtherBodyIndex :type Integer) (bFromSweep :type Boolean) (SweepResult :type Hit%20Result%20Structure%20%28by%20ref%29))
  (Utilities|Casting|CastToPRSCharacter OtherActor)
  (if (Utilities|Enum|NotEqual(Enum) (Variables|Default|GetColor) "EDC_None")
    (Class|PRSColoredDoorWorldSubsystem|AddKey (Subsystems|GetPRSColoredDoorWorldSubsystem) (Variables|Default|GetColor))
    (Audio|PlaySoundatLocation "/Game/Perspective/Art/ColoredKey/Audio/A_ColoredKey_Pickup_MSS.A_ColoredKey_Pickup_MSS" (Transformation|GetActorLocation) "0, 0, 0" 1.0 1.0 0.0 0 0 0 0)
    (Actor|DestroyActor)))

(event EventTick
  (params (DeltaSeconds :type Float%20%28single-precision%29))
  (bind _originalactorlocation (Variables|Default|GetOriginalActorLocation))
  (Transformation|SetActorLocation (Math|Vector|MakeVector (.x _originalactorlocation) (.y _originalactorlocation) (+ (* (Math|Trig|Cos(Radians) (Utilities|Time|GetTimeSeconds)) 25.0) (.z _originalactorlocation))) false false))

(event EventBeginPlay
  (Variables|Default|SetOriginalActorLocation (Transformation|GetActorLocation)))

(fn ConstructionScript
  (switch Utilities|FlowControl|Switch|SwitchonEDoorColor (Variables|Default|GetColor)
    (:EDC_None
      (Rendering|Material|SetMaterial (Variables|Debug|GetStaticMeshComponent) 0 "/Game/Perspective/Art/Shared/Materials/MI_Master.MI_Master"))
    (:EDC_Red
      (Rendering|Material|SetMaterial (Variables|Debug|GetStaticMeshComponent) 0 "/Game/Perspective/Art/ColoredKey/MI_Key_Red.MI_Key_Red"))
    (:EDC_Green
      (Rendering|Material|SetMaterial (Variables|Debug|GetStaticMeshComponent) 0 "/Game/Perspective/Art/ColoredKey/MI_Key_Green.MI_Key_Green"))
    (:EDC_Blue
      (Rendering|Material|SetMaterial (Variables|Debug|GetStaticMeshComponent) 0 "/Game/Perspective/Art/ColoredKey/MI_Key_Blue.MI_Key_Blue"))
    (:EDC_Yellow
      (Rendering|Material|SetMaterial (Variables|Debug|GetStaticMeshComponent) 0 "/Game/Perspective/Art/ColoredKey/MI_Key_Yellow.MI_Key_Yellow"))))