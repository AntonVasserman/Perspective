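; BP_ColoredGate is an interactable forcefield gate, tinted by its BagColor, that can be unlocked with a matching key.
; It listens to PRSColoredDoorWorldSubsystem, becoming passable while the current bag color matches and interactable while a matching key is held.
; A successful interaction uses the key, plays a sound and shrinks the forcefield by timeline until hidden and non-colliding.
; Highlighting outlines the frame through custom depth only when interactable.
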(event Custom|OnBagColorChanged_Event
  (params (NewBagColor :type EDoorColor%20Enum :default "EDC_None"))
  (if (Utilities|Enum|Equal(Enum) NewBagColor (Variables|Default|GetBagColor))
    (Collision|SetCollisionResponsetoAllChannels (Variables|Default|GetForcefield) "ECR_Ignore")
    (else
      (Collision|SetCollisionResponsetoAllChannels (Variables|Default|GetForcefield) "ECR_Block")))
  (Collision|SetCollisionResponsetoChannel (Variables|Default|GetForcefield) "ECC_Camera" "ECR_Ignore"))

(event Custom|OnInteractionSucceeded_Event
  (bind _forcefield (Variables|Default|GetForcefield))
  (bind _relativescale3d (Variables|/Script/Engine.SceneComponent|GetRelativeScale3D _forcefield))
  (Class|PRSColoredDoorWorldSubsystem|UseKey (Subsystems|GetPRSColoredDoorWorldSubsystem) (Variables|Default|GetBagColor))
  (Class|PRSInteractableActor|SetInteractable false)
  (Audio|PlaySoundatLocation "/Game/Perspective/Art/ColoredGate/Audio/A_ColoredDoor_Unlock_MSS.A_ColoredDoor_Unlock_MSS" (Transformation|GetActorLocation) "0, 0, 0" 1.0 1.0 0.0 0 0 0 0)
  (bind _yscale (Timeline|Fade%20Timeline Play)
    (:Update
      (Transformation|SetRelativeScale3D (Variables|Default|GetForcefield) (Math|Vector|MakeVector (.x _relativescale3d) (Math|Float|Lerp (Variables|Default|GetForcefieldOriginalScale3DY) 0.0 _yscale) (.z _relativescale3d))))
    (:Finished
      (Development|SetHiddeninGame (Variables|Default|GetForcefield) true false)
      (Collision|SetCollisionResponsetoAllChannels (Variables|Default|GetForcefield) "ECR_Ignore"))))

(event Custom|OnKeyCountChanged_Event
  (CallFunction|UpateIsInteractable))

(event EventBeginPlay
  (Rendering|SetCustomDepthStencilValue (Variables|Default|GetDoorFrame) 250)
  (CallFunction|UpateIsInteractable)
  (Variables|Default|SetForcefieldOriginalScale3DY (.y (Variables|/Script/Engine.SceneComponent|GetRelativeScale3D (Variables|Default|GetForcefield))))
  (EventDispatchers|AssignOnBagColorChanged (Subsystems|GetPRSColoredDoorWorldSubsystem) (EventDispatchers|CreateEvent :!event Custom|OnBagColorChanged_Event))
  (EventDispatchers|AssignOnKeyCountChanged (Subsystems|GetPRSColoredDoorWorldSubsystem) (EventDispatchers|CreateEvent :!event Custom|OnKeyCountChanged_Event))
  (EventDispatchers|AssignOnInteractionSucceeded (EventDispatchers|CreateEvent :!event Custom|OnInteractionSucceeded_Event)))

(event EventHighlight
  (Rendering|SetRenderCustomDepth (Variables|Default|GetDoorFrame) (Class|PRSInteractableActor|IsInteractable)))

(event EventUnHighlight
  (Rendering|SetRenderCustomDepth (Variables|Default|GetDoorFrame) false))

(fn ConstructionScript
  (bind _colormaterial (CallFunction|BagColortoColorMaterial (Variables|Default|GetBagColor)))
  (Rendering|Material|SetMaterial (Variables|Default|GetForcefield) 0 _colormaterial))

(fn BagColortoColorMaterial
  (params (BagColor :type EDoorColor%20Enum :default "EDC_None"))
  (switch Utilities|FlowControl|Switch|SwitchonEDoorColor BagColor
    (:EDC_Red
      (return "/Game/Perspective/Art/ColoredGate/Materials/MI_ColoredGate_Fill_Red.MI_ColoredGate_Fill_Red"))
    (:EDC_Green
      (return "/Game/Perspective/Art/ColoredGate/Materials/MI_ColoredGate_Fill_Green.MI_ColoredGate_Fill_Green"))
    (:EDC_Blue
      (return "/Game/Perspective/Art/ColoredGate/Materials/MI_ColoredGate_Fill_Blue.MI_ColoredGate_Fill_Blue"))
    (:EDC_Yellow
      (return "/Game/Perspective/Art/ColoredGate/Materials/MI_ColoredGate_Fill_Yellow.MI_ColoredGate_Fill_Yellow"))))

(fn UpateIsInteractable
  (bind _returnvalue (Class|PRSColoredDoorWorldSubsystem|HasKey (Subsystems|GetPRSColoredDoorWorldSubsystem) (Variables|Default|GetBagColor)))
  (Class|PRSInteractableActor|SetInteractable _returnvalue))