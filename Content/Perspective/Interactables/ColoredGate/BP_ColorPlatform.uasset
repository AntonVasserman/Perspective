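; Color platform interactable that sets the bag color in the colored door world subsystem when a PRSCharacter steps into its sphere trigger.
; The construction script applies the fill material matching the platform's Color (red, green, blue or yellow).
; It also multiplies the trigger sphere's radius by the smaller of the actor's X and Y scale.
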(event OnComponentBeginOverlap(Sphere)
  (params (OverlappedComponent :type Primitive%20Component%20Object%20Reference) (OtherActor :type Actor%20Object%20Reference) (OtherComp :type Primitive%20Component%20Object%20Reference) (OtherBodyIndex :type Integer) (bFromSweep :type Boolean) (SweepResult :type Hit%20Result%20Structure%20%28by%20ref%29))
  (Utilities|Casting|CastToPRSCharacter OtherActor)
  (Class|PRSColoredDoorWorldSubsystem|SetBagColor (Subsystems|GetPRSColoredDoorWorldSubsystem) (Variables|Default|GetColor)))

(event Collision|EventActorBeginOverlap
  (params (OtherActor :type Actor%20Object%20Reference)))

(event EventTick
  (params (DeltaSeconds :type Float%20%28single-precision%29)))

(fn ConstructionScript
  (bind _returnvalue (Transformation|GetActorScale3D))
  (Rendering|Material|SetMaterial (Variables|Default|GetPlatformFill) 0 (CallFunction|BagColortoColorMaterial (Variables|Default|GetColor)))
  (Components|Sphere|SetSphereRadius (Variables|Default|GetSphere) (* (Variables|/Script/Engine.SphereComponent|GetSphereRadius (Variables|Default|GetSphere)) (Math|Float|Min(Float) (.x _returnvalue) (.y _returnvalue))) true))

(fn BagColortoColorMaterial
  (params (BagColor :type EDoorColor%20Enum :default "EDC_None"))
  (switch Utilities|FlowControl|Switch|SwitchonEDoorColor BagColor
    (:EDC_Red
      (return "/Game/Perspective/Art/ColoredGate/Materials/MI_ColorPlatform_Fill_Red.MI_ColorPlatform_Fill_Red"))
    (:EDC_Green
      (return "/Game/Perspective/Art/ColoredGate/Materials/MI_ColorPlatform_Fill_Green.MI_ColorPlatform_Fill_Green"))
    (:EDC_Blue
      (return "/Game/Perspective/Art/ColoredGate/Materials/MI_ColorPlatform_Fill_Blue.MI_ColorPlatform_Fill_Blue"))
    (:EDC_Yellow
      (return "/Game/Perspective/Art/ColoredGate/Materials/MI_ColorPlatform_Fill_Yellow.MI_ColorPlatform_Fill_Yellow"))))