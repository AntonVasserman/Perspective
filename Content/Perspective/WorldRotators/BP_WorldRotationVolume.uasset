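; World rotation volume actor that turns its box volume, and can turn a set of objects, in animated 90-degree steps.
; A successful interaction on its Button plays a timeline that lerps BoxVolume through 90 degrees, then stores the new rotation.
; A separate RotateVolume event, not called here, precomputes each ObjectsToRotate transform pivoted around RotationArrow's forward axis, then lerps them on RotationTimeline.
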(event Custom|InteractionSucceeded
  (Variables|Default|SetNewRotation (Math|Rotator|MakeRotator (+ (.roll (Variables|Default|GetOriginalRotation)) 9e+01) (.pitch (Variables|Default|GetOriginalRotation)) (.yaw (Variables|Default|GetOriginalRotation))))
  (bind _alpha (Timeline|Timeline PlayFromStart)
    (:Update
      (Transformation|SetWorldRotation (Variables|Default|GetBoxVolume) (Math|Rotator|Lerp(Rotator) (Variables|Default|GetOriginalRotation) (Variables|Default|GetNewRotation) _alpha) false false))
    (:Finished
      (Variables|Default|SetOriginalRotation (Variables|Default|GetNewRotation)))))

(event Custom|RotateVolume
  (bind _rotationarrow (Variables|Default|GetRotationArrow))
  (bind _returnvalue (Math|Vector|GetForwardVector _rotationarrow))
  (bind _returnvalue_2 (Math|Vector|RotatorfromAxisandAngle _returnvalue 9e+01))
  (Utilities|Array|Clear (Variables|Default|GetObjectsOriginalTransform))
  (Utilities|Array|Clear (Variables|Default|GetObjectsNewTransform))
  (for _array_element (Variables|Default|GetObjectsToRotate)
    (Utilities|Array|Add (Variables|Default|GetObjectsOriginalTransform) (Transformation|GetActorTransform _array_element))
    (Utilities|Array|Add (Variables|Default|GetObjectsNewTransform) (Math|Transform|MakeTransform (+ (Transformation|GetActorLocation _array_element) (- (Math|Vector|RotateVectorAroundAxis (- (Transformation|GetActorLocation _array_element) (Transformation|GetWorldLocation (Variables|Default|GetRotationArrow))) 9e+01 (Math|Vector|GetForwardVector (Variables|Default|GetRotationArrow))) (- (Transformation|GetActorLocation _array_element) (Transformation|GetWorldLocation (Variables|Default|GetRotationArrow))))) (Math|Rotator|MakeRotator (+ (.roll (Transformation|GetActorRotation _array_element)) (.roll _returnvalue_2)) (+ (.pitch (Transformation|GetActorRotation _array_element)) (.pitch _returnvalue_2)) (+ (.yaw (Transformation|GetActorRotation _array_element)) (.yaw _returnvalue_2))) (.scale (Transformation|GetActorTransform _array_element)))))
  (bind _alpha (Timeline|Rotation%20Timeline PlayFromStart)
    (:Update
      (for (_array_element_2 _array_index) (Variables|Default|GetObjectsToRotate)
        (Transformation|SetActorTransform _array_element_2 (Math|Transform|Lerp(Transform) (Utilities|Array|Get(acopy) (Variables|Default|GetObjectsOriginalTransform) _array_index) (Utilities|Array|Get(acopy) (Variables|Default|GetObjectsNewTransform) _array_index) _alpha))))))

(event EventBeginPlay
  (EventDispatchers|BindEventtoOnInteractionSucceeded (Variables|Default|GetButton) (delegate Custom|InteractionSucceeded)))

(event Collision|EventActorBeginOverlap
  (params (OtherActor :type Actor%20Object%20Reference)))

(event EventTick
  (params (DeltaSeconds :type Float%20%28single-precision%29)))

(fn ConstructionScript)