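; BP_ColorPlatform is a colored platform that sets the active world color when something overlaps it.
; On BeginPlay it maps its Color enum to a matching red, green, blue or yellow material instance and applies it to the mesh.
; Overlapping its Box passes that color to the PRSBagColorWorldSubsystem via SetColor and prints the color name as a long-lived debug message.
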(event OnComponentBeginOverlap(Box)
  (params (OverlappedComponent :type Primitive%20Component%20Object%20Reference) (OtherActor :type Actor%20Object%20Reference) (OtherComp :type Primitive%20Component%20Object%20Reference) (OtherBodyIndex :type Integer) (bFromSweep :type Boolean) (SweepResult :type Hit%20Result%20Structure%20%28by%20ref%29))
  (Class|PRSBagColorWorldSubsystem|SetColor (Subsystems|GetPRSBagColorWorldSubsystem) (Variables|Default|GetColor))
  (Development|PrintString (Utilities|String|EnumtoString (Variables|Default|GetColor)) true true "(R=0.000000,G=0.660000,B=1.000000,A=1.000000)" 6e+02 "1"))

(event EventBeginPlay
  (Rendering|Material|SetMaterial (Variables|Debug|GetStaticMeshComponent) 0 (CallFunction|GateColortoColorMaterial (Variables|Default|GetColor))))

(event Collision|EventActorBeginOverlap
  (params (OtherActor :type Actor%20Object%20Reference)))

(event EventTick
  (params (DeltaSeconds :type Float%20%28single-precision%29)))

(fn ConstructionScript)

(fn GateColortoColorMaterial
  (params (Color :type EGateColor%20Enum :default "EGC_None"))
  (switch Utilities|FlowControl|Switch|SwitchonEGateColor Color
    (:EGC_Red
      (return "/Game/Perspective/Operatables/ColoredGate/MI_ColorPlatform_Red.MI_ColorPlatform_Red"))
    (:EGC_Green
      (return "/Game/Perspective/Operatables/ColoredGate/MI_ColorPlatform_Green.MI_ColorPlatform_Green"))
    (:EGC_Blue
      (return "/Game/Perspective/Operatables/ColoredGate/MI_ColorPlatform_Blue.MI_ColorPlatform_Blue"))
    (:EGC_Yellow
      (return "/Game/Perspective/Operatables/ColoredGate/MI_ColorPlatform_Yellow.MI_ColorPlatform_Yellow"))))