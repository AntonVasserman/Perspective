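; BP_ColoredGate is a colored gate that opens for passage when the world's active gate color matches its own GateColor.
; On BeginPlay it registers with the PRSColoredGateWorldSubsystem color-change event and switches the Gate's collision to ignore on a match or block otherwise.
; Camera and Visibility channels are always ignored after each change.
; The construction script applies a fill material chosen from GateColor (red, green, blue or yellow).
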(event Custom|OnGateColorChanged_Event
  (params (NewGateColor :type EGateColor%20Enum :default "EGC_None"))
  (if (Utilities|Enum|Equal(Enum) NewGateColor (Variables|Default|GetGateColor))
    (Collision|SetCollisionResponsetoAllChannels (Variables|Default|GetGate) "ECR_Ignore")
    (else
      (Collision|SetCollisionResponsetoAllChannels (Variables|Default|GetGate) "ECR_Block")))
  (Collision|SetCollisionResponsetoChannel (Variables|Default|GetGate) "ECC_Camera" "ECR_Ignore")
  (Collision|SetCollisionResponsetoChannel (Variables|Default|GetGate) "ECC_Visibility" "ECR_Ignore"))

(event EventBeginPlay
  (EventDispatchers|AssignOnGateColorChanged (Subsystems|GetPRSColoredGateWorldSubsystem) (delegate Custom|OnGateColorChanged_Event)))

(event Collision|EventActorBeginOverlap
  (params (OtherActor :type Actor%20Object%20Reference)))

(event EventTick
  (params (DeltaSeconds :type Float%20%28single-precision%29)))

(fn ConstructionScript
  (bind _colormaterial (CallFunction|GateColortoColorMaterial (Variables|Default|GetGateColor)))
  (Rendering|Material|SetMaterial (Variables|Default|GetGate) 0 _colormaterial))

(fn GateColortoColorMaterial
  (params (GateColor :type EGateColor%20Enum :default "EGC_Red"))
  (switch Utilities|FlowControl|Switch|SwitchonEGateColor GateColor
    (:EGC_Red
      (return "/Game/Perspective/Art/ColoredGate/Materials/MI_ColoredGate_Fill_Red.MI_ColoredGate_Fill_Red"))
    (:EGC_Green
      (return "/Game/Perspective/Art/ColoredGate/Materials/MI_ColoredGate_Fill_Green.MI_ColoredGate_Fill_Green"))
    (:EGC_Blue
      (return "/Game/Perspective/Art/ColoredGate/Materials/MI_ColoredGate_Fill_Blue.MI_ColoredGate_Fill_Blue"))
    (:EGC_Yellow
      (return "/Game/Perspective/Art/ColoredGate/Materials/MI_ColoredGate_Fill_Yellow.MI_ColoredGate_Fill_Yellow"))))