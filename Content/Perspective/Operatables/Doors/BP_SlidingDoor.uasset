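; Operatable double sliding door whose two panels part symmetrically along local Y and can automatically close once fully open.
; It listens to its own door-state dispatcher, playing a timeline forward on Opening and in reverse on Closing, with play rate scaled to the configured open duration.
; When the timeline finishes, its direction selects Open or Closed, which is broadcast, and operatability is re-enabled.
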(event Custom|DoorStateChanged
  (params (NewState :type ESlidingDoorState%20Enum :default "Closed"))
  (switch Utilities|FlowControl|Switch|SwitchonESlidingDoorState NewState
    (:Opening
      (bind (_direction _alpha) (Timeline|Door%20Opening%20Timeline PlayFromStart)
        (:Update
          (Transformation|SetRelativeLocation (Variables|Default|GetLeftDoorPanel) (Math|Vector|MakeVector 0.0 (Math|Float|Lerp 0.0 (Variables|Default|GetPanelLength) _alpha) 0.0) false false)
          (Transformation|SetRelativeLocation (Variables|Default|GetRightDoorPanel) (Math|Vector|MakeVector 0.0 (* (Math|Float|Lerp 0.0 (Variables|Default|GetPanelLength) _alpha) -1.0) 0.0) false false))
        (:Finished
          (switch Utilities|FlowControl|Switch|SwitchonETimelineDirection _direction
            (:Forward
              (bind _output_get (Variables|Default|SetCurrentState "Open"))
              (Default|CallOnDoorStateChanged _output_get)
              (if (Variables|Default|GetbCloseOnOpened)
                (bind _output_get_2 (Variables|Default|SetCurrentState "Closing"))
                (Default|CallOnDoorStateChanged _output_get_2)))
            (:Backward
              (bind _output_get_3 (Variables|Default|SetCurrentState "Closed"))
              (Default|CallOnDoorStateChanged _output_get_3)))
          (Class|PRSOperatableActor|SetOperatability true))))
    (:Closing
      (Timeline|Door%20Opening%20Timeline Reverse))))

(event EventBeginPlay
  (EventDispatchers|BindEventtoOnDoorStateChanged (delegate Custom|DoorStateChanged))
  (Components|Timeline|SetPlayRate (Variables|Default|GetDoor%20Opening%20Timeline) (/ 1.0 (Variables|Default|GetDoorOpenDuration))))

(fn ConstructionScript)