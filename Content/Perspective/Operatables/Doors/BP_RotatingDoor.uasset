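; Operatable door that rotates by a set delta over a configurable duration each time its rotation state changes to Rotating.
; A timeline, with play rate scaled to that duration, lerps the root's relative rotation to the next target.
; On finish it broadcasts the Static state, re-enables operation and computes the next target.
; Full-rotation doors keep turning the same way, while others alternate direction through a FlipFlop.
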(event Custom|RotationStateChanged
  (params (NewState :type ERotatingDoorState%20Enum :default "Static"))
  (if (Utilities|Enum|Equal(Enum) NewState "Rotating")
    (bind _alpha (Timeline|Door%20Rotation%20Timeline PlayFromStart)
      (:Update
        (Transformation|SetRelativeRotation (Variables|Default|GetDefaultSceneRoot) (Math|Rotator|Lerp(Rotator) (Variables|Default|GetOriginalRotation) (Variables|Default|GetNextRotation) _alpha) false false))
      (:Finished
        (bind _output_get (Variables|Default|SetCurrentState "Static"))
        (Default|CallOnRotationStateChanged _output_get)
        (Variables|Default|SetOriginalRotation (Variables|Default|GetNextRotation))
        (if (Variables|Default|GetbSupportFullRotation)
          (Variables|Default|SetNextRotation (Math|Rotator|CombineRotators (Variables|Default|GetOriginalRotation) (Variables|Default|GetRotationDelta)) :!label _label)
          (else
            (Utilities|FlowControl|FlipFlop
              (:A
                (Variables|Default|SetNextRotation (Math|Rotator|CombineRotators (Variables|Default|GetOriginalRotation) (* (Variables|Default|GetRotationDelta) -1.0))))
              (:B
                (goto _label)))))
        (Class|PRSOperatableActor|SetOperatability true)))))

(event EventBeginPlay
  (EventDispatchers|BindEventtoOnRotationStateChanged (delegate Custom|RotationStateChanged))
  (Components|Timeline|SetPlayRate (Variables|Default|GetDoor%20Rotation%20Timeline) (/ 1.0 (Variables|Default|GetDoorOpenDuration))))

(fn ConstructionScript)