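; BP_ElevatorPlatform is an elevator platform that travels to a destination when its child button is pressed.
; On BeginPlay it binds to the press event of the child BP_Button and hides its Borders by scaling them to zero.
; A press runs a timeline that lerps the actor to the Destination component's world location, with Borders scaled up during the ride and hidden again on arrival.
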(event Custom|MoveToDestination
  (Variables|Default|SetCurrentWorldLocation (Transformation|GetActorLocation))
  (Variables|Default|SetMoveToWorldLocation (Transformation|GetWorldLocation (Variables|Default|GetDestination)))
  (Transformation|SetWorldScale3D (Variables|Default|GetBorders) "1.000000,1.000000,1.000000")
  (bind _alpha (Timeline|MoveToDestinationTimeline Play)
    (:Update
      (Transformation|SetActorLocation (Math|Vector|Lerp(Vector) (Variables|Default|GetCurrentWorldLocation) (Variables|Default|GetMoveToWorldLocation) _alpha) false false))
    (:Finished
      (Transformation|SetWorldScale3D (Variables|Default|GetBorders) "0, 0, 0"))))

(event EventBeginPlay
  (bind _asbp_button (Utilities|Casting|CastToBP_Button (Variables|/Script/Engine.ChildActorComponent|GetChildActor (Variables|Default|GetButtonChildActor))))
  (EventDispatchers|BindEventtoOnButtonPressed _asbp_button (delegate Custom|MoveToDestination))
  (Transformation|SetWorldScale3D (Variables|Default|GetBorders) "0, 0, 0"))

(event Collision|EventActorBeginOverlap
  (params (OtherActor :type Actor%20Object%20Reference)))

(event EventTick
  (params (DeltaSeconds :type Float%20%28single-precision%29)))

(fn ConstructionScript)