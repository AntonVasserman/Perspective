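; BP_RotatingDoor is a door that animates its yaw rotation when its rotation state changes to Rotating.
; A timeline lerps the root's relative rotation toward a target rotation.
; With SupportFullRotation, each trigger adds a yaw delta and replays from start, carrying the result forward; otherwise a FlipFlop alternates playing and reversing.
; When the timeline finishes, it sets the state to Static and broadcasts the change.
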(event Custom|RotationStateChanged
  (params (NewState :type ERotatingDoorState%20Enum :default "Static"))
  (if (Utilities|Enum|Equal(Enum) NewState "Rotating")
    (if (Variables|Default|GetbSupportFullRotation)
      (Variables|Default|SetNewRotation (Math|Rotator|MakeRotator (.roll (Variables|Default|GetNewRotation)) (.pitch (Variables|Default|GetNewRotation)) (+ (.yaw (Variables|Default|GetNewRotation)) (Variables|Default|GetYawRotationDelta))))
      (bind _alpha (Timeline|Door%20Rotation%20Timeline PlayFromStart)
        (:Update
          (Transformation|SetRelativeRotation (Variables|Default|GetDefaultSceneRoot) (Math|Rotator|Lerp(Rotator) (Variables|Default|GetOriginalRotation) (Variables|Default|GetNewRotation) _alpha) false false))
        (:Finished
          (bind _output_get (Variables|Default|SetCurrentState "Static"))
          (Default|CallOnRotationStateChanged _output_get)
          (if (Variables|Default|GetbSupportFullRotation)
            (Variables|Default|SetOriginalRotation (Variables|Default|GetNewRotation)))))
      (else
        (Utilities|FlowControl|FlipFlop
          (:A
            (Timeline|Door%20Rotation%20Timeline Play))
          (:B
            (Timeline|Door%20Rotation%20Timeline Reverse)))))))

(event EventBeginPlay
  (EventDispatchers|BindEventtoOnRotationStateChanged (delegate Custom|RotationStateChanged)))

(fn ConstructionScript)