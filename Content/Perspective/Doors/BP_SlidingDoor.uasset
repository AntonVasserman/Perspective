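; Sliding door that opens and closes by animating the Z scale of its root component instead of moving it.
; It listens to its own door-state dispatcher, playing a timeline on Opening and reversing it on Closing.
; The timeline alpha becomes the absolute Z scale, while X and Y keep their values cached at BeginPlay.
; When the timeline finishes, its direction sets Open or Closed and rebroadcasts the state.
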(event Custom|DoorStateChanged
  (params (NewDoorState :type EDoorState%20Enum :default "Closed"))
  (bind _originaldoorscale3d (Variables|Default|GetOriginalDoorScale3D))
  (switch Utilities|FlowControl|Switch|SwitchonEDoorState NewDoorState
    (:Opening
      (bind (_direction _alpha) (Timeline|Door%20Opening%20Timeline Play)
        (:Update
          (Transformation|SetRelativeScale3D (Variables|Default|GetDefaultSceneRoot) (Math|Vector|MakeVector (.x _originaldoorscale3d) (.y _originaldoorscale3d) _alpha)))
        (:Finished
          (switch Utilities|FlowControl|Switch|SwitchonETimelineDirection _direction
            (:Forward
              (bind _output_get (Variables|Default|SetCurrentState "Open"))
              (Default|CallOnDoorStateChanged _output_get))
            (:Backward
              (bind _output_get_2 (Variables|Default|SetCurrentState "Closed"))
              (Default|CallOnDoorStateChanged _output_get_2))))))
    (:Closing
      (Timeline|Door%20Opening%20Timeline Reverse))))

(event EventBeginPlay
  (EventDispatchers|BindEventtoOnDoorStateChanged (delegate Custom|DoorStateChanged))
  (Variables|Default|SetOriginalDoorScale3D (Variables|/Script/Engine.SceneComponent|GetRelativeScale3D (Variables|Default|GetDefaultSceneRoot))))

(fn ConstructionScript)